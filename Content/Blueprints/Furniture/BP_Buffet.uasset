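; BP_Buffet is a furniture drop-off point where a player returns a soup order.
; When something is placed on top, it casts it to BP_Plate and, only if the plate has soup, releases the interactor's physics handle and destroys the plate.
; Its other interaction functions show a "Return order" look-at prompt and report that it holds no item and cannot spawn objects.
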(event `/Game/Blueprints/Interfaces/BPI_Interactable.PlaceOnTop`
  (params (Interactor :type "/Game/Blueprints/Chef/BP_Chef Object Reference") (ActorToPlace :type "Actor Object Reference"))
  (bind _asbp_plate (cast `/Game/Blueprints/Furniture/BP_Plate` ActorToPlace))
  (if (`/Game/Blueprints/Furniture/BP_Plate.HasSoup` _asbp_plate)
    (`PhysicsHandleComponent.ReleaseComponent` (`/Game/Blueprints/Chef/BP_Chef.PhysicsHandle` Interactor))
    (`self.K2_DestroyActor` ActorToPlace)))

(fn `CanSpawnObjects`
  (returns (CanSpawn :type Boolean))
  (return false))

(fn `CheckForItem`
  (params (Interactor :type "/Game/Blueprints/Chef/BP_Chef Object Reference"))
  (returns (HasItem :type Boolean) (ItemActor :type "Actor Object Reference") (ItemComponent :type "PrimitiveComponent Object Reference"))
  (return false null null))

(fn `LookAt`
  (params (HitComponent :type "PrimitiveComponent Object Reference"))
  (returns (LookAtActor :type "Actor Object Reference") (LookAtComponent :type "PrimitiveComponent Object Reference") (Message :type Text))
  (return self HitComponent "Return order"))

(fn `UserConstructionScript`)