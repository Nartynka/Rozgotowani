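; BP_Box is a kitchen furniture piece that dispenses ingredients to the chef and holds items placed on top.
; PlaceonTop releases the interactor's physics handle and snaps the actor to PlaceHere.
; CheckForItem scans Box overlaps for a BPI_Grabable item, skipping the held component, and caches IsHoldingItem, which blocks CanSpawnObjects when true.
; SpawnIngridient spawns ItemClassToSpawn straight into the player chef's grab; LookAt returns a placeholder message.
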(event `/Game/Blueprints/Interfaces/BPI_Interactable.PlaceOnTop`
  (params (Interactor :type "/Game/Blueprints/Chef/BP_Chef Object Reference") (ActorToPlace :type "Actor Object Reference"))
  (bind _placehere (`self.PlaceHere`))
  (`PhysicsHandleComponent.ReleaseComponent` (`/Game/Blueprints/Chef/BP_Chef.PhysicsHandle` Interactor))
  (`self.K2_SetActorLocationAndRotation` ActorToPlace (`SceneComponent.K2_GetComponentLocation` _placehere) (`SceneComponent.K2_GetComponentRotation` _placehere) false false))

(fn `CanSpawnObjects`
  (returns (CanSpawn :type Boolean))
  (return (not (`self.IsHoldingItem`))))

(fn `CheckForItem`
  (params (Interactor :type "/Game/Blueprints/Chef/BP_Chef Object Reference"))
  (returns (HasItem :type Boolean) (ItemActor :type "Actor Object Reference") (ItemComponent :type "PrimitiveComponent Object Reference"))
  (locals (Ingridient :type "Actor Object Reference") (IngridientComponent :type "PrimitiveComponent Object Reference"))
  (bind _ingridient (`local.Ingridient`))
  (bind _outoverlappingcomponents (`PrimitiveComponent.GetOverlappingComponents` (`self.Box`)))
  (if (`KismetArrayLibrary.Array_IsNotEmpty` _outoverlappingcomponents)
    (for _array_element _outoverlappingcomponents
      (if (`/Game/Blueprints/Chef/BP_Chef.IsHoldingObject` Interactor)
        (if (!= (`PhysicsHandleComponent.GetGrabbedComponent` (`/Game/Blueprints/Chef/BP_Chef.PhysicsHandle` Interactor)) _array_element)
          (bind _returnvalue (`ActorComponent.GetOwner` _array_element))
          (if (`KismetSystemLibrary.DoesImplementInterface` _returnvalue "/Game/Blueprints/Interfaces/BPI_Grabable.BPI_Grabable_C") :!label _label
            (set `local.Ingridient` _returnvalue)
            (set `local.IngridientComponent` _array_element)
            (break)))
        (else
          (goto _label))))
    (bind _output_get (set `self.IsHoldingItem` (`KismetSystemLibrary.IsValid` _ingridient)))
    (return _output_get _ingridient (`local.IngridientComponent`))))

(fn `LookAt`
  (params (HitComponent :type "PrimitiveComponent Object Reference"))
  (returns (LookAtActor :type "Actor Object Reference") (LookAtComponent :type "PrimitiveComponent Object Reference") (Message :type Text))
  (return self HitComponent "fhjdgksdujhsrhjfhdkj"))

(fn `SpawnIngridient`
  (bind _asbp_chef (cast `/Game/Blueprints/Chef/BP_Chef` (`GameplayStatics.GetPlayerCharacter` 0)))
  (bind _returnvalue (`|SpawnActorFromClass` (`self.ItemClassToSpawn`) (`KismetMathLibrary.MakeTransform` (0.0 0.0 0.0)) "Undefined" "OverrideRootScale" null null))
  (`/Game/Blueprints/Chef/BP_Chef.Grab` _asbp_chef (`/Game/Blueprints/Ingredients/BP_Ingredient.StaticMesh` _returnvalue)))

(fn `UserConstructionScript`)