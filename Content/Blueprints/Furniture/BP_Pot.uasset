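; Soup pot that takes chopped ingredients, cooks them on a stove and fills plates with the finished soup.
; Each ingredient raises the soup and lengthens cooking time, which Tick accumulates while on the stove, driving a progress widget and burning soup left too long.
; LookAt accepts plates only for full, cooked, unburned soup, and serving resets the pot.
; Older timer-based cooking logic remains unconnected in the EventGraph.
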(event `self.ReceiveBeginPlay`
  (bind _aswbp_pot_widget (cast `/Game/Blueprints/Widgets/WBP_PotWidget` (`WidgetComponent.GetWidget` (`self.ProgressBar`))))
  (set `self.PotWidget` _aswbp_pot_widget))

(event `self.ReceiveTick`
  (params (DeltaSeconds :type "Float (single-precision)"))
  (if (and (`self.ShouldCook`) (`KismetMathLibrary.Conv_IntToBool` (`self.FillLevel`)))
    (if (`self.IsCooked`)
      (set `self.BurningTime` (+ (`self.BurningTime`) DeltaSeconds))
      (else
        (set `self.BurningTime` 0.0)))
    (set `self.ElapsedCookingTime` (+ DeltaSeconds (`self.ElapsedCookingTime`)))
    (`|ExecutionSequence`
      (:`then_0`
        (if (>= (`self.FillLevel`) 3)
          (`SceneComponent.SetVisibility` (`self.Pot_Bubbles`) true false)))
      (:`then_1`
        (`self.CookOrBurn`)
        (`/Game/Blueprints/Widgets/WBP_PotWidget.Update Progress Bar` (`self.PotWidget`) (`self.ElapsedCookingTime`) (* (`self.CookTime`) (`self.FillLevel`)))))
    (else
      (`SceneComponent.SetVisibility` (`self.Pot_Bubbles`) false false))))

(event `/Game/Blueprints/Interfaces/BPI_Grabable.IsOnStove`
  (params (IsOnStove :type Boolean))
  (bind _output_get (set `self.ShouldCook` IsOnStove))
  (`SceneComponent.SetVisibility` (`self.ProgressBar`) _output_get false))

(event `Cook`
  (set `self.IsCooked` true)
  (`/Game/Blueprints/Widgets/WBP_PotWidget.CookProgressBar` (`self.PotWidget`) false))

(event `Burn`
  (`PrimitiveComponent.SetMaterial` (`self.Soup`) 0 "/Game/Blueprints/Furniture/Pot/M_Soup_Burned.M_Soup_Burned")
  (set `self.IsBurned` true)
  (`/Game/Blueprints/Widgets/WBP_PotWidget.CookProgressBar` (`self.PotWidget`) true))

(fn `AddIngridient`
  (params (GrabbedActor :type "Actor Object Reference"))
  (returns (WasAdded :type Boolean))
  (bind _asbp_plate (cast `/Game/Blueprints/Furniture/BP_Plate` GrabbedActor)
    (:`then`
      (`/Game/Blueprints/Furniture/BP_Plate.AddSoup` _asbp_plate)
      (`self.ResetSoup`))
    (:`CastFailed`
      (`/Engine/EditorBlueprintResources/StandardMacros.IncrementInt` (`self.FillLevel`)
        (:`  `
          (`SceneComponent.K2_AddRelativeLocation` (`self.Soup`) (0.0 0.0 12.0) false false)
          (`/Game/Blueprints/Widgets/WBP_PotWidget.Add Ingredient` (`self.PotWidget`) (`KismetTextLibrary.Conv_IntToText` (`self.FillLevel`)))
          (return true))))))

(fn `CookOrBurn`
  (if (>= (`self.BurningTime`) 3.0)
    (`self.Burn`)
    (elif (and (>= (`self.ElapsedCookingTime`) (* (`self.CookTime`) (`self.FillLevel`))) (not (`self.IsBurned`)))
      (`self.Cook`))))

(fn `InteractWith`
  (returns (CanGrab :type Boolean))
  (return true))

(fn `LookAt`
  (params (HitComponent :type "PrimitiveComponent Object Reference") (HoldedActor :type "Actor Object Reference"))
  (returns (CanBeLookedAtWithObject :type Boolean) (LookAtActor :type "Actor Object Reference") (LookAtComponent :type "PrimitiveComponent Object Reference") (Message :type Text))
  (locals (CanBeLooked :type Boolean :default false))
  (bind _asbp_plate (cast `/Game/Blueprints/Furniture/BP_Plate` HoldedActor)
    (:`then`
      (set `local.CanBeLooked` (and (>= (`self.FillLevel`) 3) (not (`self.IsBurned`)) (`self.IsCooked`) (not (`/Game/Blueprints/Furniture/BP_Plate.HasSoup` _asbp_plate)))))
    (:`CastFailed`
      (bind _asbp_ingredient (cast `/Game/Blueprints/Ingredients/BP_Ingredient` HoldedActor)
        (:`then`
          (set `local.CanBeLooked` (and (`/Game/Blueprints/Ingredients/BP_Ingredient.IsChopped` _asbp_ingredient) (<= (`self.FillLevel`) 3))))
        (:`CastFailed`
          _))))
  (return (`local.CanBeLooked`) self HitComponent "Click to grab! :D"))

(fn `ResetSoup`
  (set `self.FillLevel` 0)
  (set `self.IsBurned` false)
  (set `self.IsCooked` false)
  (set `self.ElapsedCookingTime` 0.0)
  (`SceneComponent.ResetRelativeTransform` (`self.Pot_Bubbles`))
  (`SceneComponent.ResetRelativeTransform` (`self.Soup`))
  (`/Game/Blueprints/Widgets/WBP_PotWidget.ResetWidget` (`self.PotWidget`))
  (`PrimitiveComponent.SetMaterial` (`self.Soup`) 0 "/Game/Blueprints/Furniture/Pot/M_Soup.M_Soup"))

(fn `UserConstructionScript`)