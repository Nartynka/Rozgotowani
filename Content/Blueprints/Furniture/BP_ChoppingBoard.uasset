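; BP_ChoppingBoard is a furniture actor that holds a grabbable ingredient for chopping and shows a "Chop something" look-at message.
; PlaceonTop releases the interactor's physics handle and snaps the actor to the PlaceHere transform.
; CheckForItem scans Box overlaps for a BPI_Grabable owner, caching the ingredient, its component and a holding flag.
; CanChopObjects returns that cached flag, while CanSpawnObjects always returns false.
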(event `/Game/Blueprints/Interfaces/BPI_Interactable.PlaceOnTop`
  (params (Interactor :type "/Game/Blueprints/Chef/BP_Chef Object Reference") (ActorToPlace :type "Actor Object Reference"))
  (bind _placehere (`self.PlaceHere`))
  (`PhysicsHandleComponent.ReleaseComponent` (`/Game/Blueprints/Chef/BP_Chef.PhysicsHandle` Interactor))
  (`self.K2_SetActorLocationAndRotation` ActorToPlace (`SceneComponent.K2_GetComponentLocation` _placehere) (`SceneComponent.K2_GetComponentRotation` _placehere) false false))

(fn `CanChopObjects`
  (returns (CanChop :type Boolean))
  (return (`self.IsHoldingItem`)))

(fn `CanSpawnObjects`
  (returns (CanSpawn :type Boolean))
  (return false))

(fn `CheckForItem`
  (returns (HasItem :type Boolean) (ItemActor :type "Actor Object Reference") (ItemComponent :type "PrimitiveComponent Object Reference"))
  (locals (Ingridient :type "Actor Object Reference") (IngridientComponent :type "PrimitiveComponent Object Reference"))
  (bind _outoverlappingcomponents (`PrimitiveComponent.GetOverlappingComponents` (`self.Box`)))
  (bind _returnvalue (`KismetArrayLibrary.Array_IsNotEmpty` _outoverlappingcomponents))
  (set `self.IsHoldingItem` _returnvalue)
  (if _returnvalue
    (for _array_element _outoverlappingcomponents
      (bind _returnvalue_2 (`ActorComponent.GetOwner` _array_element))
      (if (`KismetSystemLibrary.DoesImplementInterface` _returnvalue_2 "/Game/Blueprints/Interfaces/BPI_Grabable.BPI_Grabable_C")
        (set `local.Ingridient` _returnvalue_2)
        (set `local.IngridientComponent` _array_element)
        (break)
        (else
          (set `self.IsHoldingItem` false)))))
  (return (`self.IsHoldingItem`) (`local.Ingridient`) (`local.IngridientComponent`)))

(fn `LookAt`
  (params (HitComponent :type "PrimitiveComponent Object Reference"))
  (returns (LookAtActor :type "Actor Object Reference") (LookAtComponent :type "PrimitiveComponent Object Reference") (Message :type Text))
  (return self HitComponent "Chop something"))

(fn `UserConstructionScript`)