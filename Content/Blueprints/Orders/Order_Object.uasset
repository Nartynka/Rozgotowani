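; Order object that holds a single order's index, name, ingredients with their counts, and the interactor it belongs to.
; MakeOrder acts as an initializer, storing those values, starting a timer for the order's duration, keeping the timer handle, and returning itself.
; When the timer fires, Remove Order Object, bound by function name, tells the interactor to discard its order.
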(fn `MakeOrder`
  (params (Index :type Integer) (Name :type Text) (Ingridients :type String) (`Ingridients Count` :type Integer) (OrderTime :type "Float (single-precision)") (Interactor :type "/Game/Blueprints/Orders/BP_OrdersManager Object Reference"))
  (returns (Order :type "/Game/Blueprints/Orders/Order_Object Object Reference"))
  (set `self.Index` Index)
  (set `self.Name` Name)
  (set `self.Ingridients` Ingridients)
  (set `self.Ingridients Count` `Ingridients Count`)
  (bind _returnvalue (`KismetSystemLibrary.K2_SetTimer` null "Remove Order Object" OrderTime))
  (set `self.TimerHandle` _returnvalue)
  (set `self.Interactor` Interactor)
  (return self))

(fn `Remove Order Object`
  (`/Game/Blueprints/Orders/BP_OrdersManager.DiscardOrder` (`self.Interactor`)))